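; BP_Fighter is a scripted fighter that rolls, fires bullets alternately from two arrows on a looping timer, then burns away.
; Chained timelines drive the roll, a paper-burn dissolve on a dynamic material, and a 0-to-5 text count while destroyed.
; The count's end reverses the burn, restores the cylinders and restarts roll and fire.
; A never-reset DoOnce limits this respawn to once, so the second burn is final.
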(event Custom|Shoot
  (bind _isa (Utilities|FlowControl|FlipFlop)
    (:A
      _)
    (:B
      _))
  (Game|SpawnActorfromClass "/Game/Miniship/Gun/BP_Bullet.BP_Bullet_C" (Transformation|GetWorldTransform (select _isa (Variables|Default|GetArrow) (Variables|Default|GetArrow1))) "Undefined" "MultiplyWithRoot" 0 3.5e+04 0))

(event EventBeginPlay
  (bind _cylinder (Variables|Default|GetCylinder))
  (bind _returnvalue (Rendering|Material|CreateDynamicMaterialInstance "/Game/Levels/Catacombs/M_PaperBurn.M_PaperBurn" "None" "None" :!class /Script/Engine.KismetMaterialLibrary))
  (bind _output_get (Variables|Default|SetNewVar _returnvalue))
  (Rendering|Material|SetMaterial (Variables|Default|GetCube) 0 _output_get)
  (bind _returnvalue_2 (Utilities|Time|SetTimerbyEvent (delegate Custom|Shoot) 0.35 true :!label _label))
  (Utilities|FlowControl|DoOnce false
    (:Completed
      (bind _newtrack_0 (Timeline|Timeline PlayFromStart)
        (:Update
          (Transformation|SetRelativeRotation (Variables|Default|GetCube) (Math|Rotator|MakeRotator (Math|Float|Lerp -25.0 25.0 _newtrack_0) 0.0 0.0) false false))
        (:Finished
          (Utilities|Time|ClearandInvalidateTimerbyHandle _returnvalue_2)
          (Rendering|SetVisibility _cylinder false false)
          (bind _1 (Timeline|Timeline_0 PlayFromStart)
            (:Update
              (Rendering|Material|SetScalarParameterValue (Variables|Default|GetNewVar) "Burn" _1 :!class /Script/Engine.MaterialInstanceDynamic))
            (:Finished
              (Utilities|FlowControl|DoOnce false
                (:Completed
                  (Rendering|SetVisibility (Variables|Default|GetTextRender) true false)
                  (bind _1_2 (Timeline|Timeline_1 PlayFromStart)
                    (:Update
                      (Rendering|Components|TextRender|SetText (Variables|Default|GetTextRender) (Utilities|Text|ToText(Float) (Math|Float|Lerp 0.0 5.0 _1_2) "HalfToEven" false true 1 1 0 1)))
                    (:Finished
                      (Rendering|SetVisibility _cylinder true false)
                      (Utilities|FlowControl|Sequence
                        (:then_0
                          (Timeline|Timeline_0 ReverseFromEnd))
                        (:then_1
                          (goto _label))
                        (:then_2
                          (Timeline|Timeline PlayFromStart))
                        (:then_3
                          (Rendering|SetVisibility (Variables|Default|GetTextRender) false false))))))))))))))

(fn ConstructionScript)