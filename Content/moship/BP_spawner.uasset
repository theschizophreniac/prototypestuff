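; BP_spawner is a spawner actor that fills the area around itself with DummyShip actors in a short burst at BeginPlay.
; A looping timer fires the spawn event several times a second, and a delay clears it after five seconds.
; Each ship gets a random world-space offset in a box half as tall as it is wide, the spawner's rotation with slight random roll, and an enlarged uniform scale.
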(event Custom|tick
  (bind _returnvalue (Math|Float|MakeLiteralFloat 8.5e+03))
  (bind _spawner (Variables|Default|Getspawner))
  (bind _returnvalue_2 (Transformation|GetWorldTransform _spawner))
  (bind _returnvalue_3 (* _returnvalue -1.0))
  (Game|SpawnActorfromClass "/Game/Miniship/cluster/dummyShip.dummyShip_C" (Math|Transform|MakeTransform (+ (.location _returnvalue_2) (Math|Vector|MakeVector (Math|Random|RandomFloatinRange _returnvalue_3 _returnvalue) (Math|Random|RandomFloatinRange _returnvalue_3 _returnvalue) (Math|Random|RandomFloatinRange (/ _returnvalue_3 2.0) (/ _returnvalue 2.0)))) (Math|Rotator|CombineRotators (.rotation _returnvalue_2) (Math|Rotator|MakeRotator (Math|Random|RandomFloatinRange -25.0 25.0) 0.0 0.0)) "25.000000,25.000000,25.000000") "Undefined" "MultiplyWithRoot" 0 0))

(event EventBeginPlay
  (bind _returnvalue (Utilities|Time|SetTimerbyEvent (delegate Custom|tick) 0.2 true))
  (Utilities|FlowControl|Delay 5.0)
  (Utilities|Time|ClearandInvalidateTimerbyHandle _returnvalue))

(fn ConstructionScript)