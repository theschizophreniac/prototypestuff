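; BP_Ship is a ship actor that continuously moves forward while pitching up and down.
; Each Tick, it uses VInterpToConstant toward a point ahead along its forward vector, so it travels at Speed with a swept move.
; A game-time sine wave drives pitch while current yaw is kept, so the path undulates with the forward vector.
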(event EventTick
  (params (DeltaSeconds :type Float%20%28single-precision%29))
  (bind _returnvalue (Transformation|GetActorLocation))
  (Transformation|SetActorLocationAndRotation (Math|Interpolation|VInterptoConstant _returnvalue (+ _returnvalue (* (Transformation|GetActorForwardVector) 2e+03)) DeltaSeconds (Variables|Default|GetSpeed)) (Math|Rotator|MakeRotator 0.0 (* (Math|Trig|Sin(Radians) (* (Utilities|Time|GetGameTimeinSeconds) 0.7)) 17.5) (.yaw (Transformation|GetActorRotation))) true))

(fn ConstructionScript)