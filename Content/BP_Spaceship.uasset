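; Player ship pawn that creates its HUD, spawns an attached gun and relays controls to a second player actor.
; Input moves that actor and triggers its interaction, aims and fires the gun, or explodes a Moship on a key press.
; Each tick, velocity drives scene capture FOV and material collection speed and direction, while InputAxis mirrors ship movement values.
; BeginPlay polls for BP_2ndPlayer until found, a workaround its comment attributes to behavior living in the C++ pawn.
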(event Custom|newTerminal
  (params (NewTarget :type Texture%20Render%20Target%202D%20Object%20Reference))
  (Default|CallOnTerminalChange NewTarget))

(event EventBeginPlay
  (Utilities|FlowControl|Sequence
    (:then_0
      (bind _returnvalue (Actor|GetActorOfClass "/Game/Miniship/BP_2ndPlayer.BP_2ndPlayer_C" :!label _label)) ; this is really poorly done as i progrmamed behavior inside C++ pawn \nnot the actual player controller\n\nmay god forgive me for i have sinned
      (Utilities|IsValid _returnvalue
        (:Is%20Valid
          (Variables|Default|Set2ndPlayer _returnvalue))
        (:Is%20Not%20Valid
          (Utilities|FlowControl|RetriggerableDelay 0.2)
          (goto _label))))
    (:then_1
      (bind _returnvalue_2 (UserInterface|CreateWidget "/Game/BPW_UI.BPW_UI_C" (Game|GetPlayerController 0) self))
      (UserInterface|Viewport|AddtoViewport _returnvalue_2 0))
    (:then_2
      (CallFunction|Spawngun))))

(event EventTick
  (params (DeltaSeconds :type Float%20%28single-precision%29))
  (bind _returnvalue (Transformation|GetVelocity))
  (bind _maxthrust (Variables|Default|GetMaxThrust))
  (bind _forwardvelocity (Variables|Default|GetForwardVelocity))
  (bind _returnvalue_2 (Math|Vector|Normalize _forwardvelocity))
  (bind _returnvalue_3 (Math|Vector|VectorLength _returnvalue))
  (bind (_x _y _z) (Math|Vector|BreakVector _returnvalue_2))
  (bind _returnvalue_4 (Math|Float|NormalizetoRange _returnvalue_3 0.0 _maxthrust))
  (Variables|/Script/Engine.SceneCaptureComponent2D|SetFOVAngle (Variables|Default|GetSceneCaptureComponent2D) (Math|Float|Lerp 9e+01 1.1e+02 _returnvalue_4))
  (Rendering|Material|SetScalarParameterValue "/Game/MPC_Ship.MPC_Ship" "Speed" _returnvalue_4 :!class /Script/Engine.KismetMaterialLibrary)
  (Rendering|Material|SetVectorParameterValue "/Game/MPC_Ship.MPC_Ship" "Direction" (Utilities|Struct|MakeLinearColor _x _y _z 1.0) :!class /Script/Engine.KismetMaterialLibrary)
  (Variables|Default|SetInputAxis (Math|Vector2D|MakeVector2D (Input|AxisValues|GetMoveRight) (* (Input|AxisValues|GetMoveUp) -1.0))))

(event Input|AxisEvents|InputAxisCharacterForward
  (params (AxisValue :type Float%20%28single-precision%29))
  (Utilities|IsInput AxisValue
    (:Is%20moved?
      (Default|MoveUp (Variables|Default|Get2ndPlayer) AxisValue))))

(event Input|AxisEvents|InputAxisCharacterRight
  (params (AxisValue :type Float%20%28single-precision%29))
  (Utilities|IsInput AxisValue
    (:Is%20moved?
      (Default|MoveRight (Variables|Default|Get2ndPlayer) AxisValue))))

(event Input|AxisEvents|InputAxisShoot
  (params (AxisValue :type Float%20%28single-precision%29))
  (Utilities|IsInput AxisValue
    (:Is%20moved?
      (Default|Shoot (Variables|Default|GetGun)))))

(event Input|AxisEvents|InputAxislookX
  (params (AxisValue :type Float%20%28single-precision%29))
  (bind _gun (Variables|Default|GetGun)
    (:then
      (Utilities|IsInput AxisValue
        (:Is%20moved?
          (Default|MoveX _gun AxisValue))))
    (:else)))

(event Input|AxisEvents|InputAxisLooKY
  (params (AxisValue :type Float%20%28single-precision%29))
  (bind _gun (Variables|Default|GetGun)
    (:then
      (Utilities|IsInput AxisValue
        (:Is%20moved?
          (Default|MoveY _gun AxisValue))))
    (:else)))

(event Input|MouseEvents|RightMouseButton
  (params (Key :type Key%20Structure :default "None"))
  (:Pressed
    (Default|Interact (Variables|Default|Get2ndPlayer))))

(event Input|KeyboardEvents|1
  (params (Key :type Key%20Structure :default "None"))
  (:Pressed
    (bind _returnvalue (Actor|GetActorOfClass "/Game/moship/moship.moship_C"))
    (Default|Explod _returnvalue)))

(fn ConstructionScript)

(fn Spawngun
  (bind _returnvalue (Game|SpawnActorfromClass "/Game/Miniship/Gun/BP_Gun.BP_Gun_C" (Math|Transform|MakeTransform "0, 0, 0" "0, 0, 0" "1.000000,1.000000,1.000000") "Undefined" "MultiplyWithRoot" 0 0))
  (bind _output_get (Variables|Default|SetGun _returnvalue))
  (Transformation|AttachComponentToComponent _output_get (Variables|Default|GetGunArrow) "None" "SnapToTarget" "SnapToTarget" "KeepWorld" false))