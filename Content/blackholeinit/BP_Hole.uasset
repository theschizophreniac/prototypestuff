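; BP_Hole is a black hole actor that pulls nearby BP_Example actors toward itself and destroys those it touches.
; Each tick it applies a force from an external Gravity call to the root component of every BP_Example overlapping Influence.
; Overlapping the Eat component destroys the BP_Example.
; A local Grav function computes mass-based inverse-square attraction for physics-simulating actors, but Tick does not call it.
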(event OnComponentBeginOverlap(eat)
  (params (OverlappedComponent :type Primitive%20Component%20Object%20Reference) (OtherActor :type Actor%20Object%20Reference) (OtherComp :type Primitive%20Component%20Object%20Reference) (OtherBodyIndex :type Integer) (bFromSweep :type Boolean) (SweepResult :type Hit%20Result%20Structure%20%28by%20ref%29))
  (bind _asbp_example (Utilities|Casting|CastToBP_Example OtherActor))
  (Actor|DestroyActor _asbp_example))

(event EventBeginPlay)

(event Collision|EventActorBeginOverlap
  (params (OtherActor :type Actor%20Object%20Reference)))

(event EventTick
  (params (DeltaSeconds :type Float%20%28single-precision%29))
  (for _array_element (Collision|GetOverlappingActors (Variables|Default|Getinfluence) "/Game/blackholeinit/BP_Example.BP_Example_C" :!class /Script/Engine.PrimitiveComponent)
    (if (!= _array_element self)
      (bind _returnvalue (Class|BPCPP|Gravity _array_element self))
      (Physics|AddForce (.AsPrimitive%20Component (Utilities|Casting|CastToPrimitiveComponent (Variables|/Script/Engine.Actor|GetRootComponent _array_element))) _returnvalue "None" false))))

(fn ConstructionScript)

(fn Grav
  (params (Actor :type Actor%20Object%20Reference))
  (bind _returnvalue (Transformation|GetActorLocation))
  (bind _returnvalue_2 (Transformation|GetActorLocation Actor))
  (bind _returnvalue_3 (- _returnvalue _returnvalue_2))
  (bind _asprimitive_component (Utilities|Casting|CastToPrimitiveComponent (Variables|/Script/Engine.Actor|GetRootComponent Actor)))
  (if (Physics|IsSimulatingPhysics _asprimitive_component "None")
    (return (* (* (/ (* (Physics|GetMass _asprimitive_component) (Physics|GetMass (Variables|Default|GetSphere))) (Math|Float|Square (/ (Math|Vector|VectorLength _returnvalue_3) 1e+02))) (Variables|Default|Getconstant)) (Math|Vector|Normalize _returnvalue_3) (Utilities|Time|GetWorldDeltaSeconds)))))