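; BP_Belt is an asteroid belt spawner that fills a box volume with BP_Asteroid actors on BeginPlay.
; It spawns them in an Amount-driven loop, each at a random point within the Box extent with random rotation and non-uniform scale.
; Each asteroid's Cube gets a random mesh from RandomAsteroids, and its Sphere receives added physics velocity along the Box's right vector, starting a shared drift.
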(event EventBeginPlay
  (bind _returnvalue (Math|Random|RandomFloatinRange 0.2 3.0))
  (bind _box (Variables|Default|GetBox))
  (for _index (range 0 (Variables|Default|GetAmount))
    (bind _returnvalue_2 (Game|SpawnActorfromClass "/Game/asteroid/BP_Asteroid.BP_Asteroid_C" (Math|Transform|MakeTransform (+ (* (/ (Components|Box|GetScaledBoxExtent _box) 1.0) (Math|Vector|MakeVector (Math|Random|RandomFloatinRange -1.0 1.0) (Math|Random|RandomFloatinRange -1.0 1.0) (Math|Random|RandomFloatinRange -1.0 1.0))) (Transformation|GetWorldLocation _box)) (Math|Random|RandomRotator true) (Math|Vector|MakeVector _returnvalue _returnvalue _returnvalue)) "Undefined" "MultiplyWithRoot" 0 0))
    (Components|StaticMesh|SetStaticMesh (Variables|/Game/asteroid/BP_Asteroid.BP_Asteroid_C|GetCube _returnvalue_2) (.OutItem (Utilities|Array|Random (Variables|Default|GetrandomAsteroids))))
    (Physics|SetPhysicsLinearVelocity (Variables|/Game/asteroid/BP_Asteroid.BP_Asteroid_C|GetSphere _returnvalue_2) (* (Math|Vector|GetRightVector (Variables|Default|GetBox)) 2e+02) true "None")))

(fn ConstructionScript)