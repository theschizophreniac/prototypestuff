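; BP_Gun is a deployable miniship gun turret that aims and fires BP_Bullet projectiles, starting retracted.
; ToggleGun plays a timeline forward or backward to slide the base between positions, setting the deployed state and the scene capture's Gunner render target when finished.
; While deployed, MoveX and MoveY yaw and pitch the barrel.
; Shoot spawns bullets from ShootPoint with random angular spread, using a delay to limit fire rate by RPM.
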(event Custom|ToggleGun
  (params (On? :type Boolean))
  (Variables|Default|SetcanShoot? false)
  (if On?
    (bind (_direction _deploy) (Timeline|Deploy PlayFromStart)
      (:Update
        (Transformation|SetRelativeLocation (Variables|Default|GetBase) (Math|Vector|Lerp(Vector) "0.000000,0.000000,240.000000" "0, 0, 0" _deploy) false false))
      (:Finished
        (Variables|/Script/Engine.SceneCaptureComponent2D|SetTextureTarget (Variables|Default|GetSceneCaptureComponent2D) (Utilities|Select :Index _direction :Forward "/Game/Miniship/Gun/Gunner.Gunner" :Backward "/Game/Miniship/Gun/Gunner.Gunner"))
        (switch Utilities|FlowControl|Switch|SwitchonETimelineDirection _direction
          (:Forward
            (Variables|Default|SetDeployed? true)
            (Variables|Default|SetcanShoot? true))
          (:Backward
            (Variables|Default|SetDeployed? false)
            (Variables|Default|SetcanShoot? false)))))
    (else
      (Timeline|Deploy ReverseFromEnd))))

(event Custom|Shoot
  (bind _shootpoint (Variables|Default|GetShootPoint))
  (bind _inaccuracy (Variables|Default|Getinaccuracy))
  (bind _inaccuracy_2 (Variables|Default|Getinaccuracy))
  (bind _returnvalue (Transformation|GetWorldTransform _shootpoint))
  (if (Math|Boolean|ANDBoolean (Variables|Default|GetcanShoot?) (Variables|Default|GetDeployed?) (not (Audio|Components|Audio|IsPlaying (Variables|Default|GetDeploy))))
    (Variables|Default|SetcanShoot? false)
    (Game|SpawnActorfromClass "/Game/Miniship/Gun/BP_Bullet.BP_Bullet_C" (Math|Transform|MakeTransform (.location _returnvalue) (Math|Rotator|CombineRotators (.rotation _returnvalue) (Math|Rotator|MakeRotator 0.0 (Math|Random|RandomFloatinRange (* _inaccuracy_2 -1.0) _inaccuracy_2) (Math|Random|RandomFloatinRange (* _inaccuracy -1.0) _inaccuracy))) "1.000000,1.000000,1.000000") "AdjustIfPossibleButAlwaysSpawn" "MultiplyWithRoot" 0 (Variables|Default|GetSpeed) 0)
    (Utilities|FlowControl|Delay (/ 1.0 (/ (Variables|Default|GetRPM) 6e+01)))
    (Variables|Default|SetcanShoot? true)))

(event Custom|MoveY
  (params (Y :type Float%20%28double-precision%29))
  (if (Variables|Default|GetDeployed?)
    (Transformation|AddRelativeRotation (Variables|Default|GetBarrel) (Math|Rotator|MakeRotator 0.0 Y 0.0) false false)))

(event Custom|MoveX
  (params (X :type Float%20%28double-precision%29))
  (if (Variables|Default|GetDeployed?)
    (Transformation|AddRelativeRotation (Variables|Default|GetBarrel) (Math|Rotator|MakeRotator 0.0 0.0 X) false false)))

(event EventBeginPlay
  (CallFunction|ToggleGun false))

(fn ConstructionScript)