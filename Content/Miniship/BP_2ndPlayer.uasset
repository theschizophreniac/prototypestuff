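; BP_2ndPlayer is a second-player actor in Miniship that moves on the world XY plane and interacts with terminals.
; MoveUp and MoveRight axis inputs drive swept constant-speed interpolation along world Y and X respectively, but only while its Terminal reference is invalid.
; The interact event sends InteractMessage to every overlapping BP_Terminal; the Terminal reference is never set in this graph.
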(event Custom|MoveRight
  (params (Axis%20Value :type Float%20%28single-precision%29))
  (bind _returnvalue (Transformation|GetActorLocation))
  (Variables|Default|GetTerminal
    (:then)
    (:else
      (Transformation|SetActorLocation (Math|Interpolation|VInterptoConstant _returnvalue (+ _returnvalue (* "100.000000,0.000000,0.000000" Axis%20Value)) (Utilities|Time|GetWorldDeltaSeconds) (Variables|Default|GetSpeed)) true false))))

(event Custom|MoveUp
  (params (Axis%20Value :type Float%20%28single-precision%29))
  (bind _returnvalue (Transformation|GetActorLocation))
  (Variables|Default|GetTerminal
    (:then)
    (:else
      (Transformation|SetActorLocation (Math|Interpolation|VInterptoConstant _returnvalue (+ _returnvalue (* "0.000000,100.000000,0.000000" Axis%20Value)) (Utilities|Time|GetWorldDeltaSeconds) (Variables|Default|GetSpeed)) true false))))

(event Custom|interact
  (for _array_element (Collision|GetOverlappingActors "/Game/Miniship/BP_Terminal.BP_Terminal_C" :!class /Script/Engine.Actor)
    (Class|BPIInteract|Interact(Message) _array_element)))

(fn ConstructionScript)