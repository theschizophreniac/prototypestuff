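; BP_ShieldThing is a miniship shield that deflects bullets back the way they came.
; When an actor begins overlapping its Sphere, it prints the actor's name and continues only for a BP_Bullet.
; It swaps the bullet's material, then reverses its projectile velocity with random jitter on each axis.
; The jittered direction is not renormalized, so the scaled result only roughly preserves the original speed.
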(event OnComponentBeginOverlap(Sphere)
  (params (OverlappedComponent :type Primitive%20Component%20Object%20Reference) (OtherActor :type Actor%20Object%20Reference) (OtherComp :type Primitive%20Component%20Object%20Reference) (OtherBodyIndex :type Integer) (bFromSweep :type Boolean) (SweepResult :type Hit%20Result%20Structure%20%28by%20ref%29))
  (bind _returnvalue (Math|Random|RandomFloatinRange -0.3 0.3))
  (Development|PrintString (Utilities|GetDisplayName OtherActor))
  (bind _asbp_bullet (Utilities|Casting|CastToBP_Bullet OtherActor))
  (Rendering|Material|SetMaterial (Variables|/Game/Miniship/Gun/BP_Bullet.BP_Bullet_C|GetBullet _asbp_bullet) 0 "/Game/blackholeinit/NewMaterial2.NewMaterial2")
  (Variables|/Script/Engine.MovementComponent|SetVelocity (Variables|/Game/Miniship/Gun/BP_Bullet.BP_Bullet_C|GetProjectileMovement _asbp_bullet) (* (* (+ (Math|Vector|Normalize (Variables|/Script/Engine.MovementComponent|GetVelocity (Variables|/Game/Miniship/Gun/BP_Bullet.BP_Bullet_C|GetProjectileMovement _asbp_bullet))) (Math|Vector|MakeVector _returnvalue _returnvalue _returnvalue)) -1.0) (Math|Vector|VectorLength (Variables|/Script/Engine.MovementComponent|GetVelocity (Variables|/Game/Miniship/Gun/BP_Bullet.BP_Bullet_C|GetProjectileMovement _asbp_bullet))))))

(fn ConstructionScript)